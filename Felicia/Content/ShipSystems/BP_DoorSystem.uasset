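; BP_DoorSystem is a ship system that controls power to the ship's doors through a power cell.
; On BeginPlay it can optionally fill its Doors array with every BP_Doors actor in the level.
; Adding or removing a power cell calls the parent logic, then powers every listed door on or off.
; Tick also slowly spins its BPDoors component at a frame-rate-independent speed.
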(event EventBeginPlay
  (if (Variables|Default|GetGetAllDoorsOnStart?)
    (bind _outactors (Actor|GetAllActorsOfClass "/Game/ShipSystems/BP_Doors.BP_Doors_C"))
    (Variables|Default|SetDoors _outactors)))

(event Collision|EventActorBeginOverlap
  (params (OtherActor :type Actor%20Object%20Reference)))

(event EventTick
  (params (DeltaSeconds :type Float%20%28single-precision%29))
  (|CallParentFunction DeltaSeconds)
  (Transformation|AddLocalRotation (Variables|Default|GetBP_Doors) (* "0,1.000000, 0" DeltaSeconds) false false))

(event EventAddPowerCell
  (params (PowerCell :type BP%20Power%20Cell%20Object%20Reference))
  (|CallParentFunction PowerCell)
  (for _array_element (Variables|Default|GetDoors)
    (Default|Poweron _array_element)))

(event EventRemovePowerCell
  (|CallParentFunction)
  (for _array_element (Variables|Default|GetDoors)
    (Default|PowerOff _array_element)))

(fn ConstructionScript
  (|CallParentFunction))