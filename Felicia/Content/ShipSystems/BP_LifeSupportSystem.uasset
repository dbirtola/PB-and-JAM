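; Ship life support system that controls the oxygen level and loses the game when it runs out.
; Disengage plays the OxygenTime timeline and Engage reverses it, with oxygen set from the track value scaled to a percentage.
; At zero oxygen, the timeline's update or finish calls LoseGame on BP_FeliciaGameplayGameMode.
; An older delay-loop version of the drain and refill logic remains disconnected and never runs.
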(event EventEngage
  (|CallParentFunction)
  (Variables|Default|SetEngaged true)
  (bind _lifetime (Timeline|OxygenTime Reverse)
    (:Update
      _)
    (:Finished
      _))
  (bind _output_get (Variables|Default|SetCurrent%20Oxygen (* _lifetime 1e+02)))
  (if (<= _output_get 0.0)
    (Development|PrintString "DEAD")
    (bind _asbp_felicia_gameplay_game_mode (Utilities|Casting|CastToBP_FeliciaGameplayGameMode (Game|GetGameMode)))
    (Default|LoseGame _asbp_felicia_gameplay_game_mode "Exphysiation is best masturbation")))

(event EventDisengage
  (|CallParentFunction)
  (Variables|Default|SetEngaged false)
  (bind _lifetime (Timeline|OxygenTime Play)
    (:Update
      _)
    (:Finished
      _))
  (bind _output_get (Variables|Default|SetCurrent%20Oxygen (* _lifetime 1e+02)))
  (if (<= _output_get 0.0)
    (Development|PrintString "DEAD")
    (bind _asbp_felicia_gameplay_game_mode (Utilities|Casting|CastToBP_FeliciaGameplayGameMode (Game|GetGameMode)))
    (Default|LoseGame _asbp_felicia_gameplay_game_mode "Exphysiation is best masturbation")))

(event EventBeginPlay
  (|CallParentFunction))

(fn ConstructionScript
  (|CallParentFunction))