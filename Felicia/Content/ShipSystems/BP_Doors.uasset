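; BP_Doors is a ship-system sliding door actor with lerped movement between open and closed locations.
; BeginPlay stores the closed location, and Box overlaps by BP_FeliciaPlayerCharacter set OpeningOrClosing to 1 or -1.
; AutoOpenDoor and AutoCloseDoor, uncalled here, loop endlessly on zero Delays through LerpDoorToLocation, which zeroes that flag near the target.
; Nothing here reads the flag, and closing uses ManualDoorSpeed.
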(event OnComponentBeginOverlap(Box)
  (params (OverlappedComponent :type Primitive%20Component%20Object%20Reference) (OtherActor :type Actor%20Object%20Reference) (OtherComp :type Primitive%20Component%20Object%20Reference) (OtherBodyIndex :type Integer) (bFromSweep :type Boolean) (SweepResult :type Hit%20Result%20Structure%20%28by%20ref%29))
  (Utilities|Casting|CastToBP_FeliciaPlayerCharacter OtherActor)
  (Variables|Default|SetOpeningOrClosing 1))

(event OnComponentEndOverlap(Box)
  (params (OverlappedComponent :type Primitive%20Component%20Object%20Reference) (OtherActor :type Actor%20Object%20Reference) (OtherComp :type Primitive%20Component%20Object%20Reference) (OtherBodyIndex :type Integer))
  (Utilities|Casting|CastToBP_FeliciaPlayerCharacter OtherActor)
  (Variables|Default|SetOpeningOrClosing -1))

(event Custom|AutoOpenDoor
  (Utilities|FlowControl|Delay 0.0 :!label _label)
  (CallFunction|LerpDoortoLocation (Variables|Default|GetOpenDoorLocation) (Variables|Default|GetAutoDoorSpeed))
  (goto _label))

(event Custom|AutoCloseDoor
  (CallFunction|LerpDoortoLocation (Variables|Default|GetClosedDoorLocation) (Variables|Default|GetManualDoorSpeed) :!label _label)
  (Utilities|FlowControl|Delay 0.0)
  (goto _label))

(event EventBeginPlay
  (Variables|Default|SetClosedDoorLocation (Transformation|GetWorldLocation (Variables|Default|GetDoor))))

(event Collision|EventActorBeginOverlap
  (params (OtherActor :type Actor%20Object%20Reference)))

(event EventTick
  (params (DeltaSeconds :type Float%20%28single-precision%29)))

(fn ConstructionScript)

(fn LerpDoortoLocation
  (params (EndLocation :type Vector) (LerpSpeedAlpha :type Float%20%28single-precision%29))
  (bind _door (Variables|Default|GetDoor))
  (bind _returnvalue (Transformation|GetWorldLocation _door))
  (if (>= (Math|Vector|Distance(Vector) _returnvalue EndLocation) 1.0)
    (Transformation|SetWorldLocationAndRotation (Variables|Default|GetDoor) (Math|Vector|Lerp(Vector) _returnvalue EndLocation LerpSpeedAlpha) (Math|Rotator|Lerp(Rotator) (Transformation|GetWorldRotation _door) (Transformation|GetWorldRotation (Variables|Default|GetDefaultSceneRoot)) LerpSpeedAlpha true) false false)
    (return)
    (else
      ;[1 1 1] Exit Condition To Set Movement To Still
      (Variables|Default|SetOpeningOrClosing 0))))