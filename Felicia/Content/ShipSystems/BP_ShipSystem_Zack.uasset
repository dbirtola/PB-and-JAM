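; Ship system socket that engages while it holds a power cell and disengages when the cell is removed.
; An overlapping cell enables Tick polling until it is released, then a timeline slides it into place with physics off.
; The cell is locked briefly, then interacting with it ejects it and signals disengagement.
; A spawned voice trigger plays objective, failure, success and repeat-action lines by event name; a starting cell is optional.
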(event OnComponentBeginOverlap(Box)
  (params (OverlappedComponent :type Primitive%20Component%20Object%20Reference) (OtherActor :type Actor%20Object%20Reference) (OtherComp :type Primitive%20Component%20Object%20Reference) (OtherBodyIndex :type Integer) (bFromSweep :type Boolean) (SweepResult :type Hit%20Result%20Structure%20%28by%20ref%29))
  (if (not (Variables|Default|GetSystemActive))
    (Utilities|Casting|CastToBP_PowerCell OtherActor)
    (Utilities|FlowControl|DoOnce false
      (:Completed
        (Actor|Tick|SetActorTickEnabled true)))))

(event Custom|Engage
  (Math|Integer|IncrementInt (Variables|Default|GetNumberOfActivates)
    (:%20%20
      (Default|CallSystemEngaged))))

(event Custom|Disengage
  (Default|CallSystemDisengaged))

(event Custom|RemovePowerCell
  (EventDispatchers|UnbindEventfromInteracted (Variables|Default|GetPowerCell) (delegate Custom|RemovePowerCell))
  (Physics|SetSimulatePhysics (Variables|/Game/Interactables/BP_Pickup.BP_Pickup_C|GetSphere (Variables|Default|GetPowerCell)) true)
  (Variables|Default|SetPowerCell 0)
  (Variables|Default|SetSystemActive false)
  (Actor|Tick|SetActorTickEnabled true)
  (CallFunction|Disengage)
  (bind _curve_for_add (Timeline|Timeline_0 Stop)
    (:Update
      _)
    (:Finished
      _))
  (Utilities|IsValid (Variables|Default|GetPowerCell)
    (:Is%20Valid
      (Transformation|SetWorldLocation (Variables|/Game/Interactables/BP_Pickup.BP_Pickup_C|GetSphere (Variables|Default|GetPowerCell)) (Math|Vector|Lerp(Vector) (Variables|Default|GetPowerCellInitialLoc) (Math|Transform|TransformLocation (Transformation|GetWorldTransform (Variables|Default|GetBox)) (Variables|Default|GetPowerCellLocation)) _curve_for_add) false false))))

(event Custom|AddPowerCell
  (params (PowerCell :type BP%20Power%20Cell%20Object%20Reference))
  (bind _output_get (Variables|Default|SetPowerCell PowerCell))
  (Physics|SetSimulatePhysics (Variables|/Game/Interactables/BP_Pickup.BP_Pickup_C|GetSphere _output_get) false)
  (Variables|Default|SetSystemActive true)
  (Default|SetIsInteractable (Variables|Default|GetPowerCell) false)
  (Utilities|Time|SetTimerbyEvent (delegate Custom|Make%20Power%20Cell%20Interactable%20Again) (Variables|Default|GetCell%20Lockout%20Time))
  (EventDispatchers|BindEventtoInteracted (Variables|Default|GetPowerCell) (delegate Custom|RemovePowerCell))
  (Variables|Default|SetPowerCellInitialLoc (Transformation|GetActorLocation (Variables|Default|GetPowerCell)))
  (CallFunction|Engage)
  (bind _curve_for_add (Timeline|Timeline_0 PlayFromStart)
    (:Update
      _)
    (:Finished
      _))
  (Utilities|IsValid (Variables|Default|GetPowerCell)
    (:Is%20Valid
      (Transformation|SetWorldLocation (Variables|/Game/Interactables/BP_Pickup.BP_Pickup_C|GetSphere (Variables|Default|GetPowerCell)) (Math|Vector|Lerp(Vector) (Variables|Default|GetPowerCellInitialLoc) (Math|Transform|TransformLocation (Transformation|GetWorldTransform (Variables|Default|GetBox)) (Variables|Default|GetPowerCellLocation)) _curve_for_add) false false))))

(event Custom|Play%20Cue%20By%20Event
  (params (Name :type E_AudioEvent%20Enum :default "NewEnumerator0"))
  (switch Utilities|FlowControl|Switch|SwitchonE_AudioEvent Name
    (:NewEnumerator0
      (Development|PrintString "Playing Begin Audio")
      (Default|TriggerObjectiveVoice (Variables|Default|GetVoiceTrigger))
      (if (Variables|Default|GetSystemActive)
        (Default|CallSystemEngaged)))
    (:NewEnumerator1
      (Development|PrintString "Playing Fail Audio")
      (Default|TriggerFailureVoice (Variables|Default|GetVoiceTrigger)))
    (:NewEnumerator3
      (Development|PrintString "Playing Success audio")
      (Default|TriggerSuccessVoice (Variables|Default|GetVoiceTrigger)))
    (:NewEnumerator2
      (Development|PrintString "Playing Repetitive Audio")
      (Default|TriggerUnnecessaryVoice (Variables|Default|GetVoiceTrigger)))))

(event Custom|Make%20Power%20Cell%20Interactable%20Again
  (bind _powercell (Variables|Default|GetPowerCell)
    (:then
      (Default|SetIsInteractable _powercell true))
    (:else)))

(event EventBeginPlay
  (bind _returnvalue (Game|SpawnActorfromClass "/Game/Audio/BP_VoiceTrigger.BP_VoiceTrigger_C" (Math|Transform|MakeTransform "0, 0, 0" "0, 0, 0" "1,1,1") "Undefined" 0 0))
  (bind _output_get (Variables|Default|SetVoiceTrigger _returnvalue))
  (Variables|/Game/Audio/BP_VoiceTrigger.BP_VoiceTrigger_C|SetVoices _output_get (Variables|Default|GetVoices))
  (if (Variables|Default|GetStartWithPowerCell)
    (bind _returnvalue_2 (Game|SpawnActorfromClass "/Game/Interactables/BP_PowerCell.BP_PowerCell_C" (Math|Transform|MakeTransform (Transformation|GetWorldLocation (Variables|Default|GetBox)) "0, 0, 0" "1,1,1") "Undefined" 0 0))
    (CallFunction|AddPowerCell _returnvalue_2)
    (else
      (CallFunction|Disengage))))

(event EventTick
  (params (DeltaSeconds :type Float%20%28single-precision%29))
  (bind _cell (Utilities|PowerCellPresent?)
    (:Yes
      (if (not (Variables|/Game/Interactables/BP_Pickup.BP_Pickup_C|GetHeld _cell))
        (CallFunction|AddPowerCell _cell)
        (Actor|Tick|SetActorTickEnabled false :!label _label)
        (Utilities|FlowControl|DoOnce false) ; enters at Reset
      ))
    (:No
      (goto _label))))

(fn ConstructionScript)