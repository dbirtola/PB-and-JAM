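; BPC_PowerSlot is a ship systems Blueprint that, in this graph, only provides particle and audio helper events, with no power logic.
; SpawnParticles spawns a given emitter, and PlayOneShot spawns an AmbientSound actor at world origin, ignoring its Looping input.
; The other events drive a shared Audio component: play with optional interruption of current sound, stop, and fade in or out.
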(event Custom|SpawnParticles
  (params (NewParam :type Particle%20System%20Object%20Reference))
  (Effects|SpawnEmitteratLocation NewParam "0, 0, 0"))

(event Custom|PlayOneShot
  (params (SFX :type Sound%20Wave%20Object%20Reference) (Looping? :type Boolean))
  (bind _returnvalue (Game|SpawnActorfromClass "/Script/Engine.AmbientSound" (Math|Transform|MakeTransform "0, 0, 0") "Undefined" 0 0))
  (Audio|Components|Audio|SetSound (Variables|/Script/Engine.AmbientSound|GetAudioComponent _returnvalue) SFX)
  (Audio|Components|Audio|Play (Variables|/Script/Engine.AmbientSound|GetAudioComponent _returnvalue) 0.0))

(event Custom|PlayAudio
  (params (NewSound :type Sound%20Wave%20Object%20Reference) (OverwriteOldAudio? :type Boolean))
  (bind _audio (Variables|Default|GetAudio))
  (if OverwriteOldAudio?
    (Audio|Components|Audio|SetSound _audio NewSound :!label _label)
    (Audio|Components|Audio|Play _audio 0.0)
    (elif (not (Audio|Components|Audio|IsPlaying _audio))
      (goto _label))))

(event Custom|StopAudio
  (Audio|Components|Audio|Stop (Variables|Default|GetAudio)))

(event Custom|FadeOutAudio
  (params (FadeOutDuration :type Float%20%28single-precision%29))
  (Audio|Components|Audio|FadeOut (Variables|Default|GetAudio) FadeOutDuration 0.0 :!class /Script/Engine.AudioComponent))

(event Custom|FadeInAndPlayAudio
  (params (New%20Sound :type Sound%20Wave%20Object%20Reference) (FadeInDuration :type Float%20%28single-precision%29))
  (bind _audio (Variables|Default|GetAudio))
  (Audio|Components|Audio|SetSound _audio New%20Sound)
  (Audio|Components|Audio|FadeIn _audio FadeInDuration 1.0 0.0 :!class /Script/Engine.AudioComponent))

(event EventBeginPlay)

(event EventTick
  (params (DeltaSeconds :type Float%20%28single-precision%29)))