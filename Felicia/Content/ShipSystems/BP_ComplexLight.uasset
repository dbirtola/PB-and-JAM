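; BP_ComplexLight is a ship-system light that randomly flickers its spot and point lights, extending a parent light class with a TurnOff event.
; A timer starts the first flicker after a random delay on BeginPlay, then a timeline curve with random noise drives both intensities.
; Timeline updates re-arm a fixed-delay timer to repeat the flicker, and TurnOff clears it.
; A second timeline feeds the random range but never runs.
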(event Custom|RandomFlicker
  (bind _smoothflicker (Timeline|Timeline_00 PlayFromStart)
    (:Update
      (Rendering|Components|Light|SetIntensity (Variables|Default|GetSpot) (* (Math|Random|RandomFloatinRange _smoothflicker (Math|Random|RandomFloatinRange (stale _smoothflicker) 0.8)) (* _smoothflicker 1e+03)))
      (bind _returnvalue (Utilities|Time|SetTimerbyEvent (delegate Custom|RandomFlicker) 5.0))
      (Variables|Default|SetFlickerTimerHandle _returnvalue))))

(event EventBeginPlay
  (|CallParentFunction)
  (bind _returnvalue (Utilities|Time|SetTimerbyEvent (delegate Custom|RandomFlicker) (Math|Random|RandomFloatinRange 4.0 8.0)))
  (Variables|Default|SetFlickerTimerHandle _returnvalue))

(event Collision|EventActorBeginOverlap
  (params (OtherActor :type Actor%20Object%20Reference))
  (|CallParentFunction OtherActor) ; This node is disabled and will not be called.\nDrag off pins to build functionality.
)

(event EventTick
  (params (DeltaSeconds :type Float%20%28single-precision%29))
  (|CallParentFunction DeltaSeconds) ; This node is disabled and will not be called.\nDrag off pins to build functionality.
)

(event EventTurnOff
  (|CallParentFunction)
  (Utilities|Time|ClearandInvalidateTimerbyHandle (Variables|Default|GetFlickerTimerHandle)))

(fn ConstructionScript
  (|CallParentFunction))