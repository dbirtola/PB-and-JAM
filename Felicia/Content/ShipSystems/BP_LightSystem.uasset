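; BP_LightSystem is a ship system that switches a set of BP_SimpleLight actors on and off.
; With GetAllLightsOnStart set, BeginPlay fills the Lights array with every BP_SimpleLight in the level; parent BeginPlay runs only on that branch.
; Engage and Disengage call their parent versions, then loop over Lights calling TurnOn or TurnOff.
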(event EventBeginPlay
  (if (Variables|Default|GetGetAllLightsOnStart)
    (bind _outactors (Actor|GetAllActorsOfClass "/Game/ShipSystems/BP_SimpleLight.BP_SimpleLight_C"))
    (Variables|Default|SetLights _outactors)
    (|CallParentFunction)))

(event EventEngage
  (|CallParentFunction)
  (for _array_element (Variables|Default|GetLights)
    (Default|Turnon _array_element)))

(event EventDisengage
  (|CallParentFunction)
  (for _array_element (Variables|Default|GetLights)
    (Default|TurnOff _array_element)))

(fn ConstructionScript
  (|CallParentFunction))