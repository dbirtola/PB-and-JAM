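; BP_SimpleLight is a light Blueprint under ShipSystems that switches a point light on and off.
; TurnOn and TurnOff events set the PointLight intensity directly to a fixed brightness or zero.
; Flicker support is unfinished: its event and function are empty, and the looping timer, timeline-driven intensity curve and LightOn branch are disconnected and never run.
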(event Custom|TurnOn
  (Rendering|Components|Light|SetIntensity (Variables|Default|GetPointLight) 5e+03))

(event Custom|TurnOff
  (Rendering|Components|Light|SetIntensity (Variables|Default|GetPointLight) 0.0))

(event Custom|FlickerLightsRandomly)

(event EventBeginPlay)

(event Collision|EventActorBeginOverlap
  (params (OtherActor :type Actor%20Object%20Reference)))

(event EventTick
  (params (DeltaSeconds :type Float%20%28single-precision%29)))

(fn ConstructionScript)

(fn FlickeringLights)