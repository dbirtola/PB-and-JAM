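; Ship gravity system that switches the player character between normal gravity and a floaty low-gravity state.
; Disengage lowers gravity scale, air control and walk speed, gives a tiny upward launch, then starts a timeline that drives gravity scale.
; When the timeline finishes, it repeats the nudge and replays, looping the fluctuation.
; Engage counts activations, restores movement values and stops the timeline.
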(event Collision|EventActorBeginOverlap
  (params (OtherActor :type Actor%20Object%20Reference)))

(event EventTick
  (params (DeltaSeconds :type Float%20%28single-precision%29))
  (|CallParentFunction DeltaSeconds) ; This node is disabled and will not be called.\nDrag off pins to build functionality.
)

(event EventEngage
  (bind _charactermovement (Variables|Default|GetCharacterMovement))
  (Math|Integer|IncrementInt (Variables|Default|GetNumberOfActivates)
    (:%20%20
      (Variables|/Script/Engine.CharacterMovementComponent|SetGravityScale _charactermovement 1.0)
      (Variables|/Script/Engine.CharacterMovementComponent|SetAirControl _charactermovement 0.05)
      (Variables|/Script/Engine.CharacterMovementComponent|SetAirControlBoostMultiplier _charactermovement 2.0)
      (Variables|/Script/Engine.CharacterMovementComponent|SetAirControlBoostVelocityThreshold _charactermovement 25.0)
      (Variables|/Script/Engine.CharacterMovementComponent|SetMaxWalkSpeed _charactermovement 6e+02)
      (bind _gravity (Timeline|Timeline_1 Stop)
        (:Update
          (Variables|/Script/Engine.CharacterMovementComponent|SetGravityScale (Variables|Default|GetCharacterMovement) _gravity))
        (:Finished
          (Utilities|FlowControl|Delay 0.0)
          (Character|LaunchCharacter (Game|GetPlayerCharacter 0) (Math|Vector|MakeVector 0.0 0.0 0.01) false false)
          (Timeline|Timeline_1 PlayFromStart))))))

(event EventDisengage
  (bind _charactermovement (Variables|Default|GetCharacterMovement))
  (Character|LaunchCharacter (Game|GetPlayerCharacter 0) (Math|Vector|MakeVector 0.0 0.0 0.01) false false)
  (Variables|/Script/Engine.CharacterMovementComponent|SetGravityScale _charactermovement 0.2)
  (Variables|/Script/Engine.CharacterMovementComponent|SetAirControl _charactermovement 0.0)
  (Variables|/Script/Engine.CharacterMovementComponent|SetAirControlBoostMultiplier _charactermovement 0.0)
  (Variables|/Script/Engine.CharacterMovementComponent|SetAirControlBoostVelocityThreshold _charactermovement 0.0)
  (Variables|/Script/Engine.CharacterMovementComponent|SetMaxWalkSpeed (Variables|Default|GetCharacterMovement) 2e+02)
  (bind _gravity (Timeline|Timeline_1 PlayFromStart)
    (:Update
      (Variables|/Script/Engine.CharacterMovementComponent|SetGravityScale (Variables|Default|GetCharacterMovement) _gravity))
    (:Finished
      (Utilities|FlowControl|Delay 0.0)
      (Character|LaunchCharacter (Game|GetPlayerCharacter 0) (Math|Vector|MakeVector 0.0 0.0 0.01) false false)
      (Timeline|Timeline_1 PlayFromStart))))

(event EventBeginPlay
  (Variables|Default|SetCharacterMovement (Variables|/Script/Engine.Character|GetCharacterMovement (Game|GetPlayerCharacter 0)))
  (|CallParentFunction))

(fn ConstructionScript
  (|CallParentFunction))