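; BP_FeliciaGameplayGameMode is a game mode for critical ship-system events and the loss condition.
; A looping timer picks a random CriticalEvents table row, but the result is currently unused.
; A single loss timer tracks one target system, reporting success if it is active on expiry, otherwise failure and showing the end-game menu.
; A request during a valid timer only invalidates the handle and warns, without starting a new timer.
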(event Custom|Lose%20Game
  (params (Loss%20Reason :type String))
  (bind _returnvalue (Game|GetPlayerController 0))
  (Development|PrintString (Utilities|String|Append "Player lost!: [Reason]: " Loss%20Reason))
  (bind _returnvalue_2 (UserInterface|CreateWidget "/Game/UI/Menus/EndGameMenu.EndGameMenu_C" _returnvalue))
  (UserInterface|Viewport|AddtoViewport _returnvalue_2 0)
  (Variables|/Script/Engine.PlayerController|SetbShowMouseCursor _returnvalue true))

(event Custom|Set%20Loss%20Timer%20For%20System
  (params (Time :type Float%20%28single-precision%29) (Ship%20System :type BP%20Ship%20System%20Object%20Reference))
  (Variables|Default|SetCurrent%20Target%20System Ship%20System)
  (Development|PrintString (Utilities|String|Append "Setting loss timer for: " (Utilities|String|ToString(Float) Time)))
  (if (Utilities|Time|IsValidTimerHandle (Variables|Default|GetLoss%20Timer%20Handle))
    (Utilities|Time|InvalidateTimerHandle (Variables|Default|GetLoss%20Timer%20Handle))
    (Development|PrintString "Loss timer triggered while another loss timer was in progress. Was this intentional?? Talk to Damen!. Unless hes in a meeting. ")
    (else
      (bind _returnvalue (Utilities|Time|SetTimerbyEvent (delegate Custom|On%20Loss%20Timer%20Expired) Time))
      (Variables|Default|SetLoss%20Timer%20Handle _returnvalue))))

(event Custom|On%20Loss%20Timer%20Expired
  (if (Variables|/Game/ShipSystems/BP_ShipSystem.BP_ShipSystem_C|GetSystemActive (Variables|Default|GetCurrent%20Target%20System))
    (Development|PrintString (Utilities|String|Append "System " (Utilities|GetDisplayName (Variables|Default|GetCurrent%20Target%20System)) " not active in time. Player losing game"))
    (Default|CallSystemSucceeded)
    (else
      (Development|PrintString (Utilities|String|Append "System " (Utilities|GetDisplayName (Variables|Default|GetCurrent%20Target%20System)) " not active in time. Player losing game"))
      (Default|CallSystemFailed)
      (CallFunction|LoseGame "Out of Time"))))

(event Custom|GenerateRandomEvent
  (bind _criticalevents (Variables|Default|GetCriticalEvents))
  (bind _outrownames (DataTable|GetDataTableRowNames _criticalevents))
  (bind _returnvalue (Utilities|GetDataTableRow _criticalevents (Utilities|Array|Get(acopy) _outrownames (Math|Random|RandomIntegerinRange 0 (- (Utilities|Array|Length _outrownames) 1))))))

(event Custom|Generate%20Event
  (CallFunction|GenerateRandomEvent))

(event Custom|Set%20Loss%20Timer%20for%20All%20Systems%20of%20Type
  (params (Ship%20System%20Type :type BP%20Ship%20System%20Class%20Reference))
  (bind _outactors (Actor|GetAllActorsOfClass Ship%20System%20Type))
  (for _array_element _outactors
    (CallFunction|SetLossTimerforSystem 0.0 _array_element)))

(event EventBeginPlay
  (Utilities|Time|SetTimerbyEvent (delegate Custom|Generate%20Event) 2e+01 true))

(fn ConstructionScript
  (|CallParentFunction))