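; BP_VoiceTrigger plays random voiceover lines for four situations: objective, success, failure and unnecessary.
; Each Trigger function passes its own sound list to SendRandomVoiceover, which picks a sound wave and hands it to Speaker.PlayNewVoiceover.
; The event graph and construction script are empty, so playback depends on the Trigger functions being called.
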(event EventBeginPlay)

(event Collision|EventActorBeginOverlap
  (params (OtherActor :type Actor%20Object%20Reference)))

(event EventTick
  (params (DeltaSeconds :type Float%20%28single-precision%29)))

(fn ConstructionScript)

(fn TriggerObjectiveVoice
  (Utilities|SendRandomVoiceover (Variables|Default|GetObjectiveVoices)))

(fn TriggerSuccessVoice
  (Utilities|SendRandomVoiceover (Variables|Default|GetSuccessVoices)))

(fn TriggerFailureVoice
  (Utilities|SendRandomVoiceover (Variables|Default|GetFailureVoices)))

(fn TriggerUnnecessaryVoice
  (Utilities|SendRandomVoiceover (Variables|Default|GetUnnecessaryVoices)))