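; BP_Speaker is an actor that plays voiceover lines and shows their subtitles, starting with B0_Cue on BeginPlay.
; PlayNewVoiceover plays a line directly when idle; if audio is playing, it switches to a random InBetweens cue and stores the new line as pending.
; OnAudioFinished then plays the pending line.
; Subtitles go immediately to BP_Dialogue via the Dialogue_text actor, even for queued lines.
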(event OnAudioFinished(voiceoverPlayer)
  (if (Variables|Default|GetsoundWaiting)
    (Utilities|PlayNewSoundCue (Variables|Default|GetvoiceoverPlayer) (Variables|Default|GetnextSound)
      (:%20%20
        (Variables|Default|SetsoundWaiting false)))))

(event EventBeginPlay
  (CallFunction|PlayNewVoiceover "/Game/Audio/Sounds/b0_Cue.b0_Cue"))

(event Collision|EventActorBeginOverlap
  (params (OtherActor :type Actor%20Object%20Reference)))

(event EventTick
  (params (DeltaSeconds :type Float%20%28single-precision%29)))

(fn ConstructionScript)

(fn PlayNewVoiceover
  (params (New%20Sound :type Sound%20Cue%20Object%20Reference))
  (bind _voiceoverplayer (Variables|Default|GetvoiceoverPlayer))
  (if (Audio|Components|Audio|IsPlaying (Variables|Default|GetvoiceoverPlayer))
    (bind _selectedsound (Utilities|GetRandomSoundCue (Variables|Default|GetInBetweens))
      (:%20%20
        (Utilities|PlayNewSoundCue _voiceoverplayer _selectedsound
          (:%20%20
            (Variables|Default|SetnextSound New%20Sound)
            (Variables|Default|SetsoundWaiting true)))))
    (else
      (Utilities|PlayNewSoundCue _voiceoverplayer New%20Sound
        (:%20%20
          _))))
  (bind _returnvalue (Actor|GetActorOfClass "/Game/Audio/dialogue_text.dialogue_text_C"))
  (bind _asbp_dialogue (Utilities|Casting|CastToBP_Dialogue (Variables|/Game/Audio/dialogue_text.dialogue_text_C|GetDialogueWidget _returnvalue)))
  (Default|DisplaySubtitle _asbp_dialogue New%20Sound))