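; BP_FeliciaPlayerCharacter is a first-person player character that can grab and release pickup objects.
; The capsule collider stores any overlapped BP_Pickup, and ending the overlap does not clear it.
; Pressing G calls Interact on the stored pickup and releasing it calls UnInteract, guarded by a Grab flag.
; An unconnected camera line trace with a PhysicsHandle grab remains in the graph but never runs.
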(event OnComponentBeginOverlap(CapsuleCollider)
  (params (OverlappedComponent :type Primitive%20Component%20Object%20Reference) (OtherActor :type Actor%20Object%20Reference) (OtherComp :type Primitive%20Component%20Object%20Reference) (OtherBodyIndex :type Integer) (bFromSweep :type Boolean) (SweepResult :type Hit%20Result%20Structure%20%28by%20ref%29))
  (bind _asbp_pickup (Utilities|Casting|CastToBP_Pickup OtherActor))
  (Variables|Default|SetPickup _asbp_pickup))

(event OnComponentEndOverlap(CapsuleCollider)
  (params (OverlappedComponent :type Primitive%20Component%20Object%20Reference) (OtherActor :type Actor%20Object%20Reference) (OtherComp :type Primitive%20Component%20Object%20Reference) (OtherBodyIndex :type Integer)))

(event EventBeginPlay)

(event Collision|EventActorBeginOverlap
  (params (OtherActor :type Actor%20Object%20Reference)))

(event EventTick
  (params (DeltaSeconds :type Float%20%28single-precision%29)))

(event Input|KeyboardEvents|G
  (params (Key :type Key%20Structure :default "None"))
  (bind _self self)
  (bind _pickup (Variables|Default|GetPickup))
  (:Pressed
    (if (not (Variables|Default|GetGrab?))
      (Utilities|IsValid _pickup
        (:Is%20Valid
          (Variables|Default|SetGrab? true)
          (Default|Interact _pickup _self)))))
  (:Released
    (if (Variables|Default|GetGrab?)
      (Utilities|IsValid _pickup
        (:Is%20Valid
          (Variables|Default|SetGrab? false)
          (Default|UnInteract _pickup _self))))))

(fn ConstructionScript
  (|CallParentFunction))