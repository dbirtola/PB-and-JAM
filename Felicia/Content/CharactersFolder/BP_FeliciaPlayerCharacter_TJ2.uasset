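; Felicia player character that toggles between normal and low gravity and interacts with pickups.
; Keys 2 and 3 switch gravity, changing air control and walk speed, with a looping timeline driving gravity scale.
; Capsule overlap stores a pickup for hold-Enter interaction, while "wall"-tagged overlaps raise low-gravity speed.
; A custom hit handler, with no caller shown, reflects velocity off non-floor surfaces; physics-handle grab code is disconnected.
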(event OnComponentBeginOverlap(CapsuleCollider)
  (params (OverlappedComponent :type Primitive%20Component%20Object%20Reference) (OtherActor :type Actor%20Object%20Reference) (OtherComp :type Primitive%20Component%20Object%20Reference) (OtherBodyIndex :type Integer) (bFromSweep :type Boolean) (SweepResult :type Hit%20Result%20Structure%20%28by%20ref%29))
  (bind _asbp_pickup (Utilities|Casting|CastToBP_Pickup OtherActor))
  (Variables|Default|SetPickup _asbp_pickup))

(event OnComponentEndOverlap(CapsuleCollider)
  (params (OverlappedComponent :type Primitive%20Component%20Object%20Reference) (OtherActor :type Actor%20Object%20Reference) (OtherComp :type Primitive%20Component%20Object%20Reference) (OtherBodyIndex :type Integer)))

(event EventBeginPlay)

(event Collision|EventActorBeginOverlap
  (params (OtherActor :type Actor%20Object%20Reference))
  (if (Actor|ActorHasTag OtherActor "wall")
    (if (Variables|Default|GetGravityEnable)
      (Variables|/Script/Engine.CharacterMovementComponent|SetMaxWalkSpeed (Variables|Character|GetCharacterMovement) 3.5e+02)
      (Variables|Default|SetonWall true))))

(event Collision|EventActorEndOverlap
  (params (OtherActor :type Actor%20Object%20Reference))
  (if (Actor|ActorHasTag OtherActor "wall")
    (if (Variables|Default|GetGravityEnable)
      (Variables|/Script/Engine.CharacterMovementComponent|SetMaxWalkSpeed (Variables|Character|GetCharacterMovement) 2e+02)
      (Variables|Default|SetonWall false))))

(event EventTick
  (params (DeltaSeconds :type Float%20%28single-precision%29))
  (Variables|Default|SetBounce "0, 0, 0")
  (Variables|Default|SetBounced? false))

(event Input|KeyboardEvents|2
  (params (Key :type Key%20Structure))
  (:Pressed
    (CallFunction|AntiGrav)))

(event Input|KeyboardEvents|Enter
  (params (Key :type Key%20Structure))
  (bind _self self)
  (bind _pickup (Variables|Default|GetPickup))
  (:Pressed
    (if (not (Variables|Default|GetGrab?))
      (Utilities|IsValid _pickup
        (:Is%20Valid
          (Variables|Default|SetGrab? true)
          (Default|Interact _pickup _self)))))
  (:Released
    (if (Variables|Default|GetGrab?)
      (Utilities|IsValid _pickup
        (:Is%20Valid
          (Variables|Default|SetGrab? false)
          (Default|UnInteract _pickup _self))))))

(event Input|KeyboardEvents|3
  (params (Key :type Key%20Structure))
  (:Pressed
    (CallFunction|EnableGravity)))

(event Custom|EnableGravity
  (bind _charactermovement (Variables|Character|GetCharacterMovement))
  ;[1 1 1] Enable Gravity
  (Variables|/Script/Engine.CharacterMovementComponent|SetGravityScale _charactermovement 1.0)
  (Variables|/Script/Engine.CharacterMovementComponent|SetAirControl _charactermovement 0.05)
  (Variables|/Script/Engine.CharacterMovementComponent|SetAirControlBoostMultiplier _charactermovement 2.0)
  (Variables|/Script/Engine.CharacterMovementComponent|SetAirControlBoostVelocityThreshold _charactermovement 25.0)
  (Variables|/Script/Engine.CharacterMovementComponent|SetMaxWalkSpeed _charactermovement 6e+02)
  (Variables|Default|SetGravityEnable false)
  ;[1 1 1] Anti Gravity
  (bind _gravity (Timeline|Timeline_0 Stop)
    (:Update
      (Variables|/Script/Engine.CharacterMovementComponent|SetGravityScale (Variables|Character|GetCharacterMovement) _gravity))
    (:Finished
      (Utilities|FlowControl|Delay 0.0)
      (Character|LaunchCharacter (Math|Vector|MakeVector 0.0 0.0 0.01) false false)
      (Timeline|Timeline_0 PlayFromStart))))

(event Custom|AntiGrav
  (bind _charactermovement (Variables|Character|GetCharacterMovement))
  (bind _charactermovement_2 (Variables|Character|GetCharacterMovement))
  ;[1 1 1] Anti Gravity
  (Character|LaunchCharacter (Math|Vector|MakeVector 0.0 0.0 0.01) false false)
  (Variables|/Script/Engine.CharacterMovementComponent|SetGravityScale _charactermovement_2 0.2)
  (Variables|/Script/Engine.CharacterMovementComponent|SetAirControl _charactermovement_2 0.0)
  (Variables|/Script/Engine.CharacterMovementComponent|SetAirControlBoostMultiplier _charactermovement_2 0.0)
  (Variables|/Script/Engine.CharacterMovementComponent|SetAirControlBoostVelocityThreshold _charactermovement_2 0.0)
  (Variables|Default|SetGravityEnable true)
  (if (Variables|Default|GetonWall)
    (Variables|/Script/Engine.CharacterMovementComponent|SetMaxWalkSpeed _charactermovement 3.5e+02)
    (bind _gravity (Timeline|Timeline_0 PlayFromStart)
      (:Update
        (Variables|/Script/Engine.CharacterMovementComponent|SetGravityScale (Variables|Character|GetCharacterMovement) _gravity))
      (:Finished
        (Utilities|FlowControl|Delay 0.0)
        (Character|LaunchCharacter (Math|Vector|MakeVector 0.0 0.0 0.01) false false)
        (Timeline|Timeline_0 PlayFromStart)))
    (else
      (Variables|/Script/Engine.CharacterMovementComponent|SetMaxWalkSpeed _charactermovement 2e+02)
      (Timeline|Timeline_0 PlayFromStart))))

(event Custom|CustomEvent
  (params (MyComp :type Primitive%20Component%20Object%20Reference) (Other :type Actor%20Object%20Reference) (OtherComp :type Primitive%20Component%20Object%20Reference) (bSelfMoved :type Boolean) (HitLocation :type Vector) (HitNormal :type Vector) (NormalImpulse :type Vector) (Hit :type Hit%20Result%20Structure%20%28by%20ref%29))
  (bind _charactermovement (Variables|Character|GetCharacterMovement))
  (bind _returnvalue (Pawn|Components|CharacterMovement|GetLastUpdateVelocity _charactermovement))
  ;[1 1 1] Bouncing
  (if (Variables|Default|GetGravityEnable)
    (if (not (Math|Vector|Equal(Vector) HitNormal "0, 0,1.000000" 0.0001))
      (Variables|Default|SetBounced? true)
      (bind _output_get (Variables|Default|SetBounce (+ _returnvalue (* (* HitNormal (Math|Vector|DotProduct _returnvalue HitNormal)) -2.0))))
      (Character|LaunchCharacter _output_get true true))))

(fn ConstructionScript
  (|CallParentFunction))